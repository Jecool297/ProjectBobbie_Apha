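; BP_HautFond is a shoal obstacle that reacts when the player's boat enters its box.
; TypeDeFonds selects the effect: type 0 fires the boat's first-collision event once, other types slow it through linear damping.
; In tutorial mode, type 0 also eases boat health down each tick while damping it and updating the UI, then grants immunity at the target.
; Leaving the box clears the damping.
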(event `self.ReceiveBeginPlay`
  (bind _asbp_boat_template (cast `/Game/Blueprints/Boats/Bobbie/BP_BoatTemplate` (`GameplayStatics.GetPlayerPawn` 0)))
  (set `self.As BP Boat Template` _asbp_boat_template))

(event `VieBasseTutoriel`
  (params (TargetVie :type "Float (double-precision)"))
  (bind _as_bp_boat_template (`self.As BP Boat Template`))
  (bind _sm_bobbie (`/Game/Blueprints/Boats/Bobbie/BP_BoatTemplate.SM_Bobbie` _as_bp_boat_template))
  (bind _output_get (set `/Game/Blueprints/Boats/Bobbie/BP_BoatTemplate.SanteBobbie` (`KismetMathLibrary.FInterpTo` (`/Game/Blueprints/Boats/Bobbie/BP_BoatTemplate.SanteBobbie` _as_bp_boat_template) TargetVie (`GameplayStatics.GetWorldDeltaSeconds`) 2.0) _as_bp_boat_template))
  (if (<= _output_get TargetVie)
    (set `/Game/Blueprints/Boats/Bobbie/BP_BoatTemplate.Immunise?` true _as_bp_boat_template)
    (`PrimitiveComponent.SetLinearDamping` _sm_bobbie 0.0)
    (else
      (`/Game/Widget/Hud/WBP_UI_Jeu.MiseAJourVie` (`/Game/Blueprints/Boats/Bobbie/BP_BoatTemplate.UI_EnJeu` _as_bp_boat_template))
      (`PrimitiveComponent.SetLinearDamping` _sm_bobbie 2.0))))

(event `self.ReceiveTick`
  (params (DeltaSeconds :type "Float (single-precision)"))
  (if (`self.DansLaZone`)
    (set `self.Delta Seconds` (+ (`self.Delta Seconds`) DeltaSeconds))
    (if (`self.Tutoriel?`)
      (if (== (`self.Type De Fonds`) 0)
        (`self.VieBasseTutoriel` 50.0)))
    (else
      (set `self.Delta Seconds` 0.0))))

(event `self.Box.OnComponentBeginOverlap`
  (params (OverlappedComponent :type "PrimitiveComponent Object Reference") (OtherActor :type "Actor Object Reference") (OtherComp :type "PrimitiveComponent Object Reference") (OtherBodyIndex :type Integer) (bFromSweep :type Boolean) (SweepResult :type "HitResult Structure (by ref)"))
  (bind _as_bp_boat_template (`self.As BP Boat Template`))
  (if (== OtherActor _as_bp_boat_template)
    (set `self.DansLaZone` true)
    (if (== (`self.Type De Fonds`) 0)
      (`/Engine/EditorBlueprintResources/StandardMacros.DoOnce` false
        (:`Completed`
          (`/Game/Blueprints/Boats/Bobbie/BP_BoatTemplate.PremiereCollision` _as_bp_boat_template)))
      (else
        (`self.Ralentissement`)))))

(event `Ralentissement`
  (`PrimitiveComponent.SetLinearDamping` (`/Game/Blueprints/Boats/Bobbie/BP_BoatTemplate.SM_Bobbie` (`self.As BP Boat Template`)) 2.5))

(event `self.Box.OnComponentEndOverlap`
  (params (OverlappedComponent :type "PrimitiveComponent Object Reference") (OtherActor :type "Actor Object Reference") (OtherComp :type "PrimitiveComponent Object Reference") (OtherBodyIndex :type Integer))
  (bind _as_bp_boat_template (`self.As BP Boat Template`))
  (if (== OtherActor _as_bp_boat_template)
    (set `self.DansLaZone` false)
    (`PrimitiveComponent.SetLinearDamping` (`/Game/Blueprints/Boats/Bobbie/BP_BoatTemplate.SM_Bobbie` _as_bp_boat_template) 0.0)))

(fn `UserConstructionScript`
  (switch `/Game/Blueprints/Obstacle/Enum_TypeDeFond` (`self.Type De Fonds`)))