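; Pickup actor that the player's boat collects by touching its sphere trigger.
; On the first overlap with the player pawn, the collectable eases up to a fixed relative height and a timeline drives its uniform scale.
; When the timeline ends, it plays a success sound, calls AjoutCollectable on the BP_BoatTemplate pawn cached at BeginPlay, then destroys itself.
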(event `self.ReceiveBeginPlay`
  (bind _asbp_boat_template (cast `/Game/Blueprints/Boats/Bobbie/BP_BoatTemplate` (`GameplayStatics.GetPlayerPawn` 0)))
  (set `self.As BP Boat Template` _asbp_boat_template))

(event `self.Sphere.OnComponentBeginOverlap`
  (params (OverlappedComponent :type "PrimitiveComponent Object Reference") (OtherActor :type "Actor Object Reference") (OtherComp :type "PrimitiveComponent Object Reference") (OtherBodyIndex :type Integer) (bFromSweep :type Boolean) (SweepResult :type "HitResult Structure (by ref)"))
  (bind _collectable (`self.Collectable`))
  (if (== OtherActor (`GameplayStatics.GetPlayerPawn` 0))
    (`/Engine/EditorBlueprintResources/StandardMacros.DoOnce` false
      (:`Completed`
        (`KismetSystemLibrary.MoveComponentTo` _collectable (0.0 0.0 550.0) (`SceneComponent.RelativeRotation` _collectable) true true 0.34)
        (bind (_direction _newtrack_0) (`Timeline|ExplodingCollectable`)
          (:`Update`
            (bind _returnvalue (* _newtrack_0 0.5))
            (`SceneComponent.SetRelativeScale3D` (`self.Collectable`) (`KismetMathLibrary.MakeVector` _returnvalue _returnvalue _returnvalue)))
          (:`Finished`
            (`GameplayStatics.PlaySound2D` "/Game/Sfx/Sons/Effects/Success/Sfx_Succes001.Sfx_Succes001" 1.0 1.0 0.0 null null)
            (`/Game/Blueprints/Boats/Bobbie/BP_BoatTemplate.AjoutCollectable` (`self.As BP Boat Template`))
            (`self.K2_DestroyActor`)))))))

(fn `UserConstructionScript`)