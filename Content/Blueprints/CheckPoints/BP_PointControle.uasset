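; BP_PointControle is a checkpoint actor that the player's boat crosses to advance an objective counter in the in-game UI.
; It caches the player boat at BeginPlay, and an InitialisationUI event fetches the objective counter widget from that boat's UI.
; When the boat overlaps its box, it plays a success sound once, notifies the counter via ObjectifFranchi and destroys itself.
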(event `self.ReceiveBeginPlay`
  (bind _asbp_boat_template (cast `/Game/Blueprints/Boats/Bobbie/BP_BoatTemplate` (`GameplayStatics.GetPlayerPawn` 0)))
  (set `self.As BP Boat Template` _asbp_boat_template))

(event `InitialisationUI`
  (set `self.UI Objectif ` (`/Game/Blueprints/CheckPoints/BP_PointControle.WBP_CompteurObjectif` (`.UI_EnJeu` (`/Game/Blueprints/Boats/Bobbie/BP_BoatTemplate.UI_EnJeu` (`self.As BP Boat Template`))))))

(event `self.Box.OnComponentBeginOverlap`
  (params (OverlappedComponent :type "PrimitiveComponent Object Reference") (OtherActor :type "Actor Object Reference") (OtherComp :type "PrimitiveComponent Object Reference") (OtherBodyIndex :type Integer) (bFromSweep :type Boolean) (SweepResult :type "HitResult Structure (by ref)"))
  (if (== OtherActor (`self.As BP Boat Template`))
    (`/Engine/EditorBlueprintResources/StandardMacros.DoOnce` false
      (:`Completed`
        (`GameplayStatics.PlaySound2D` "/Game/Sfx/Sons/Effects/Success/Sfx_Sucess002.Sfx_Sucess002" 1.0 1.0 0.0 null null)
        (`/Game/Widget/Mission/WBP_CompteurObjectif.ObjectifFranchi` (`self.UI Objectif `))
        (`self.K2_DestroyActor`)))))

(fn `UserConstructionScript`)