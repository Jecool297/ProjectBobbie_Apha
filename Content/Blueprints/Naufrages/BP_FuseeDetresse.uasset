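; Distress flare actor for shipwrecks that rises on spawn and can show a countdown for the player's rescue window.
; BeginPlay starts the Niagara effect, eases the flare upward and creates the WBP_Timer widget.
; Once ActiverTimer runs, Tick shrinks the effect as time drains and flags the critical final stretch.
; At expiry it disables the player boat's movement, shows the time-out message and destroys the parent wreck.
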(event `GetNaufrageParent`
  (params (NaufrageParent :type "Actor Object Reference"))
  (set `self.Reference Naufrage Parent` NaufrageParent))

(event `self.ReceiveTick`
  (params (DeltaSeconds :type "Float (single-precision)"))
  (bind _bp_bobbie_ref (`self.BP_Bobbie_ref`))
  (if (`self.TimerLance?`)
    ;[1 1 1] Initialise le Timer une fois le feu lancé en l'air
    (`SceneComponent.SetRelativeScale3D` (`self.Niagara1`) (`KismetMathLibrary.Conv_DoubleToVector` (`KismetMathLibrary.MapRangeClamped` (`KismetMathLibrary.Conv_IntToDouble` (`self.Timer`)) (`self.TempsMax`) 0.0 100.0 1.0)))
    (bind _output_get (set `self.Compteur` (+ (`self.Compteur`) (`GameplayStatics.GetWorldDeltaSeconds`))))
    (bind _output_get_2 (set `self.Timer` (`KismetMathLibrary.Round` (- (`self.TempsMax`) _output_get))))
    (if (<= _output_get_2 0)
      (`/Engine/EditorBlueprintResources/StandardMacros.DoOnce` false
        (:`Completed`
          (`/Game/Blueprints/Boats/Bobbie/BP_BoatTemplate.DesactiverMouvements` _bp_bobbie_ref)
          (`/Game/Widget/Hud/WBP_UI_Jeu.MessageTempsEcoule` (`/Game/Blueprints/Boats/Bobbie/BP_BoatTemplate.UI_EnJeu` _bp_bobbie_ref) "Visible")
          (bind _reference_naufrage_parent (`self.Reference Naufrage Parent`)
            (:`then`
              (`self.K2_DestroyActor` _reference_naufrage_parent))
            (:`else`))))
      (elif (<= _output_get_2 60)
        (`/Engine/EditorBlueprintResources/StandardMacros.DoOnce` false
          (:`Completed`
            (`/Game/Widget/Hud/WBP_Timer.CouleurTempsCritique` (`self.TimerRef`))))))))

(event `self.ReceiveBeginPlay`
  (`self.ActivateFlareVfx`)
  (`|ExecutionSequence`
    (:`then_0`
      (`KismetSystemLibrary.Delay` 0.2)
      (`self.LancerFeuDetresse`))
    (:`then_1`
      (bind _returnvalue (`KismetMaterialLibrary.CreateDynamicMaterialInstance` "/Game/Material/Instances/Vfx/MI_FlareLight.MI_FlareLight"))
      (set `self.MaterialFusee_Ref` _returnvalue)
      (`self.LancerTimer`))))

(event `ActivateFlareVfx`
  ;[1 1 1] Comment
  (`ActorComponent.Activate` (`self.Niagara1`) false))

(event `ActiverTimer`
  (if (`self.Timer?`)
    (set `self.TimerLance?` true)
    (`/Game/Widget/Hud/WBP_Timer.TrouverParent` (`self.TimerRef`) self)))

(event `LancerTimer`
  (if (`self.Timer?`)
    (bind _returnvalue (`|CreateWidget` "/Game/Widget/Hud/WBP_Timer.WBP_Timer_C"))
    (bind _output_get (set `self.TimerRef` _returnvalue))
    (`WidgetComponent.SetWidget` (`self.TempsRestant`) _output_get)
    (bind _asbp_boat_template (cast `/Game/Blueprints/Boats/Bobbie/BP_BoatTemplate` (`GameplayStatics.GetPlayerPawn` 0)))
    (set `self.BP_Bobbie_ref` _asbp_boat_template)))

(event `LancerFeuDetresse`
  (`KismetSystemLibrary.MoveComponentTo` (`self.EffetFeuDetresse`) (`self.HauteurFeuDetresse`) (struct) true false 2.0))

(event `Cacher_AfficherFX`
  (params (bNewVisibility :type Boolean))
  (`SceneComponent.SetVisibility` (`self.Niagara`) bNewVisibility false)
  (`SceneComponent.SetVisibility` (`self.Niagara1`) bNewVisibility false)
  (`SceneComponent.SetVisibility` (`self.TempsRestant`) bNewVisibility false))

(fn `UserConstructionScript`)