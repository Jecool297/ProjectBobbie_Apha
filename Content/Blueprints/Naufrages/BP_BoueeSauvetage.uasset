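; Lifebuoy-throw rescue minigame actor, placed at the boat's current shipwreck (Naufrage), where the player must time the throw.
; The buoy oscillates between two markers at random speeds while a three-point Niagara arc tracks its distance to the boat.
; Throwing inside the ideal zone updates rescue count, objectives, base and UI, then repossesses the boat and destroys buoy and wreck.
; A miss briefly shows text; cancel returns to the boat.
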(event `self.ReceiveTick`
  (params (DeltaSeconds :type "Float (single-precision)"))
  (bind _positiontrajectoire (`self.PositionTrajectoire`))
  (bind _returnvalue (`KismetMathLibrary.Vector_Distance` (`SceneComponent.K2_GetComponentLocation` (`self.SM_BoueeSauvetage`)) (`self.K2_GetActorLocation` (`self.As BP Boat Template`))))
  (bind _returnvalue_2 (* _returnvalue -1.0))
  (`/Engine/EditorBlueprintResources/StandardMacros.IsValid` (`self.As BP Boat Template`)
    (:`Is Valid`
      (`KismetArrayLibrary.Array_Set` _positiontrajectoire)
      (`KismetArrayLibrary.Array_Set` _positiontrajectoire 1 (`KismetMathLibrary.MakeVector` 0.0 (/ _returnvalue_2 2.0) (/ _returnvalue 2.0)))
      (`KismetArrayLibrary.Array_Set` _positiontrajectoire 2 (`KismetMathLibrary.MakeVector` 0.0 _returnvalue_2))
      (`NiagaraDataInterfaceArrayFunctionLibrary.SetNiagaraArrayVector` (`self.AimingLine `) "User.PositionParticules" _positiontrajectoire))))

(event `self.ReceiveBeginPlay`
  (bind (_returnvalue_x _returnvalue_y _returnvalue_z) (`KismetMathLibrary.BreakVector` (`SceneComponent.K2_GetComponentLocation` (`self.SM_BoueeSauvetage`))))
  (bind _returnvalue (`GameplayStatics.GetActorOfClass` "/Game/Blueprints/Boats/Bobbie/BP_BoatTemplate.BP_BoatTemplate_C"))
  (bind _output_get (set `self.As BP Boat Template` _returnvalue))
  (bind (_returnvalue_x_2 _returnvalue_y_2) (`KismetMathLibrary.BreakVector` (`self.K2_GetActorLocation` (`/Game/Blueprints/Boats/Bobbie/BP_BoatTemplate.CurrentNaufrage` _output_get))))
  ;[1 1 1] Place la jauge à l'emplacement du naufrage
  (`SceneComponent.K2_SetWorldLocation` (`self.AimingWidget`) (- (`KismetMathLibrary.MakeVector` _returnvalue_x_2 _returnvalue_y_2 _returnvalue_z) (0.0 0.0 10.0)) false false)
  (`self.EnableInput` (`GameplayStatics.GetPlayerController` 0))
  (bind _returnvalue_2 (`PrimitiveComponent.CreateDynamicMaterialInstance` (`self.SM_BoueeSauvetage`) 0 "/Game/Art/Buoy/SmallBuoy/Materials/MI_SafetyBuoy.MI_SafetyBuoy" "None"))
  (bind _output_get_2 (set `self.MaterailBouee` _returnvalue_2))
  (`MaterialInstanceDynamic.SetScalarParameterValue` _output_get_2 "HologramTransition" 0.0)
  (`self.BoueeAvant`))

(event `LancerBouee`
  (bind _textrender (`self.TextRender`))
  (bind _as_bp_boat_template (`self.As BP Boat Template`))
  (bind _as_bp_boat_template_2 (`self.As BP Boat Template`))
  (bind _as_bp_boat_template_3 (`self.As BP Boat Template`))
  (bind _as_bp_boat_template_4 (`self.As BP Boat Template`))
  (if (`self.TirReussi`) :!label _label
    (`MaterialInstanceDynamic.SetScalarParameterValue` (`self.MaterailBouee`) "HologramTransition" 1.0)
    (`self.StopMouvement `)
    (`|ExecutionSequence`
      (:`then_0`
        (`KismetSystemLibrary.Delay` 0.5)
        (bind _asbp_naufrage_v2 (cast `/Game/Blueprints/Naufrages/BP_NaufrageV2` (`/Game/Blueprints/Boats/Bobbie/BP_BoatTemplate.CurrentNaufrage` _as_bp_boat_template_2)))
        (bind _asbp_base (cast `/Game/Blueprints/Base/BP_Base` (`/Game/Blueprints/Boats/Bobbie/BP_BoatTemplate.CurrentBase` _as_bp_boat_template_2)))
        (`KismetArrayLibrary.Array_RemoveItem` (`/Game/Blueprints/Base/BP_Base.NaufrageA Recuperer` _asbp_base) _asbp_naufrage_v2)
        (`self.K2_DestroyActor` (`/Game/Blueprints/Naufrages/BP_NaufrageV2.FeuDetresse_Ref` _asbp_naufrage_v2))
        (set `/Game/Blueprints/Boats/Bobbie/BP_BoatTemplate.IndexPersonneSecouru` (+ (`/Game/Blueprints/Boats/Bobbie/BP_BoatTemplate.IndexPersonneSecouru` _as_bp_boat_template_3) 1) _as_bp_boat_template_3)
        (set `/Game/Blueprints/Naufrages/BP_NaufrageV2.ObjectifActuelle` false _asbp_naufrage_v2)
        (`/Game/Blueprints/Naufrages/BP_NaufrageV2.ChangerObjectif` _asbp_naufrage_v2)
        (`/Game/Widget/Hud/WBP_UI_Jeu.AjouterNaufrage` (`/Game/Blueprints/Boats/Bobbie/BP_BoatTemplate.UI_EnJeu` _as_bp_boat_template) "Sauvé!")
        (`/Game/Widget/Hud/WBP_LevierVitesse.SnapLevierNeutre` (`/Game/Widget/Hud/WBP_UI_Jeu.WBP_LevierVitesse` (`/Game/Blueprints/Boats/Bobbie/BP_BoatTemplate.UI_EnJeu` _as_bp_boat_template)))
        (bind _asbp_base_2 (cast `/Game/Blueprints/Base/BP_Base` (`/Game/Blueprints/Boats/Bobbie/BP_BoatTemplate.CurrentBase` _as_bp_boat_template)))
        (if (== (`/Game/Blueprints/Base/BP_Base.PersonnesRequises` _asbp_base_2) (`/Game/Blueprints/Boats/Bobbie/BP_BoatTemplate.IndexPersonneSecouru` _as_bp_boat_template))
          (bind _aswbp_compte_naufrage (cast `/Game/Widget/Mission/WBP_CompteNaufrage` (`WidgetComponent.GetWidget` (`/Game/Blueprints/Base/BP_Base.Widget` _asbp_base_2))))
          (`/Game/Widget/Mission/WBP_CompteNaufrage.SetPersonneRecuperer` _aswbp_compte_naufrage)
          (`/Game/Blueprints/Base/BP_Base.AffichageZoneNaufrage` _asbp_base_2 true)
          (`KismetSystemLibrary.Delay` 0.1)
          (`self.K2_DestroyActor` self)
          (`self.K2_DestroyActor` (`/Game/Blueprints/Boats/Bobbie/BP_BoatTemplate.CurrentNaufrage` _as_bp_boat_template))
          (else
            (`KismetSystemLibrary.Delay` 0.1)
            (`self.K2_DestroyActor` self)
            (`self.K2_DestroyActor` (`/Game/Blueprints/Boats/Bobbie/BP_BoatTemplate.CurrentNaufrage` _as_bp_boat_template)))))
      (:`then_1`
        (`/Game/Blueprints/Boats/Bobbie/BP_BoatTemplate.Repossess` _as_bp_boat_template_4 false)
        (`/Game/Widget/Hud/WBP_ModeVisee.CloseNotification` (`/Game/Widget/Hud/WBP_UI_Jeu.WBP_ModeVisee` (`/Game/Blueprints/Boats/Bobbie/BP_BoatTemplate.UI_EnJeu` _as_bp_boat_template_4)))
        (`/Game/Widget/Hud/WBP_TableauDeBord.CacherTout` (`/Game/Widget/Hud/WBP_UI_Jeu.WBP_TableauDeBord` (`/Game/Blueprints/Boats/Bobbie/BP_BoatTemplate.UI_EnJeu` (`self.As BP Boat Template`))))
        (`KismetSystemLibrary.Delay` 0.5)
        (`/Game/Blueprints/GuidingArrow/BP_FlecheGuide.AffichageFleche` (`/Game/Blueprints/Boats/Bobbie/BP_BoatTemplate.Ref_FlecheGuide` (`self.As BP Boat Template`)) true)))
    (else
      (`TextRenderComponent.K2_SetText` _textrender (`self.Value`))
      (`SceneComponent.SetVisibility` _textrender true false)
      (`KismetSystemLibrary.Delay` 2.0)
      (`SceneComponent.SetVisibility` _textrender false false))))

(event `EnhancedInput|/Game/Controls/Inputs/ControleBouee/IA_Lancer`
  (params (ActionValue :type Boolean) (ElapsedSeconds :type "Float (double-precision)") (TriggeredSeconds :type "Float (double-precision)") (InputAction :type "InputAction Object Reference" :default "/Game/Controls/Inputs/ControleBouee/IA_Lancer.IA_Lancer"))
  (:`Started`
    (goto _label)))

(event `EnhancedInput|/Game/Controls/Inputs/ControleBateau/IA_Cancel-Back`
  (params (ActionValue :type Boolean) (ElapsedSeconds :type "Float (double-precision)") (TriggeredSeconds :type "Float (double-precision)") (InputAction :type "InputAction Object Reference" :default "/Game/Controls/Inputs/ControleBateau/IA_Cancel-Back.IA_Cancel-Back"))
  (bind _as_bp_boat_template (`self.As BP Boat Template`))
  (:`Started`
    (`/Game/Blueprints/Boats/Bobbie/BP_BoatTemplate.Repossess` (`self.As BP Boat Template`) true :!label _label_2)
    (`/Game/Widget/Hud/WBP_UI_Jeu.DansLaZoneSauvetage` (`/Game/Blueprints/Boats/Bobbie/BP_BoatTemplate.UI_EnJeu` (`self.As BP Boat Template`)))
    (`/Game/Widget/Hud/WBP_TableauDeBord.AfficherSauvetage` (`/Game/Widget/Hud/WBP_UI_Jeu.WBP_TableauDeBord` (`/Game/Blueprints/Boats/Bobbie/BP_BoatTemplate.UI_EnJeu` _as_bp_boat_template)))
    (`KismetSystemLibrary.Delay` 0.5)
    (`/Game/Blueprints/GuidingArrow/BP_FlecheGuide.AffichageFleche` (`/Game/Blueprints/Boats/Bobbie/BP_BoatTemplate.Ref_FlecheGuide` _as_bp_boat_template) true)
    (`self.K2_DestroyActor`)))

(event `BoueeAvant`
  (bind _returnvalue (`KismetMathLibrary.RandomFloatInRange` 1.0 2.0))
  (bind _sm_boueesauvetage (`self.SM_BoueeSauvetage`))
  ;[1 1 1] Mouvement de la bouee à vitesse variante
  (`KismetSystemLibrary.MoveComponentTo` _sm_boueesauvetage (`SceneComponent.RelativeLocation` (`self.FinZone`)) (struct :`Pitch` -90.0) true true _returnvalue :!label _label_3)
  (`KismetSystemLibrary.Delay` 0.2)
  (`KismetSystemLibrary.MoveComponentTo` _sm_boueesauvetage (`SceneComponent.RelativeLocation` (`self.DebutZone`)) (struct :`Pitch` -90.0) true true _returnvalue :!label _label_4)
  (goto _label_3))

(event `StopMouvement`
  ;[1 1 1] Mouvement de la bouee à vitesse variante
  (`|ExecutionSequence`
    (:`then_0`
      (goto _label_3 :!via `Stop`))
    (:`then_1`
      (goto _label_4 :!via `Stop`))))

(event `CancelModeSauvetage`
  (goto _label_2))

(event `self.ZoneIdeal.OnComponentBeginOverlap`
  (params (OverlappedComponent :type "PrimitiveComponent Object Reference") (OtherActor :type "Actor Object Reference") (OtherComp :type "PrimitiveComponent Object Reference") (OtherBodyIndex :type Integer) (bFromSweep :type Boolean) (SweepResult :type "HitResult Structure (by ref)"))
  ;[1 1 1] Comment
  (if (or (== OtherComp (`self.Cible`)) (== (`self.SM_BoueeSauvetage`) OtherComp))
    (set `self.TirReussi` true)))

(event `self.ZoneIdeal.OnComponentEndOverlap`
  (params (OverlappedComponent :type "PrimitiveComponent Object Reference") (OtherActor :type "Actor Object Reference") (OtherComp :type "PrimitiveComponent Object Reference") (OtherBodyIndex :type Integer))
  (if (or (== OtherComp (`self.Cible`)) (== (`self.SM_BoueeSauvetage`) OtherComp))
    (set `self.TirReussi` false)))

(fn `UserConstructionScript`
  (`TextRenderComponent.K2_SetText` (`self.TextRender`) ""))