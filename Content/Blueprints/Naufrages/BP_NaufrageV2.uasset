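; Castaway rescue point for the player's boat, Bobbie, with a rescue zone and a life buoy.
; Entering the zone sets Bobbie's rescue state and shows mobile or PC UI, optionally after a movement-pausing tutorial; leaving clears both.
; Events launch a distress flare, toggle smoke and advance the guide arrow; functions count rescues and resize the zone ring.
; A hit buoy returns via ACRetourPosition; the force-based slowdown logic is disconnected.
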(event `self.ReceiveTick`
  (params (DeltaSeconds :type "Float (single-precision)")))

(event `self.ReceiveBeginPlay`
  ;[1 1 1] Enregistrement de la position initiale
  (set `self.TransformationInitiale` (`self.GetTransform`))
  ;[1 1 1] Référence à Bobbie
  (bind _asbp_boat_template (cast `/Game/Blueprints/Boats/Bobbie/BP_BoatTemplate` (`GameplayStatics.GetPlayerPawn` 0)))
  (set `self.Bobbie_Ref` _asbp_boat_template)
  (`self.EnableInput` (`GameplayStatics.GetPlayerController` 0))
  (bind _returnvalue (`GameplayStatics.GetActorOfClass` "/Game/Blueprints/GuidingArrow/BP_FlecheGuide.BP_FlecheGuide_C"))
  (set `self.FlecheGuideObjectif_Ref` _returnvalue)
  (`SceneComponent.SetHiddenInGame` (`self.BoueeSauvetage`) true true))

(event `self.BoueeSauvetage.OnComponentHit`
  (params (HitComponent :type "PrimitiveComponent Object Reference") (OtherActor :type "Actor Object Reference") (OtherComp :type "PrimitiveComponent Object Reference") (NormalImpulse :type "Vector Structure") (Hit :type "HitResult Structure (by ref)"))
  ;[1 1 1] Retour à la position initial 3 secondes après l'impacte avec tout objet.
  (`/Game/Blueprints/Buoy/Parent/AC_RetourPosition.Collision_Hit` (`self.AC_RetourPosition`) (`self.TransformationInitiale`) (`self.BoueeSauvetage`) (`self.Duree Deplacement`)))

(event `self.ZoneDeRalentissement.OnComponentBeginOverlap`
  (params (OverlappedComponent :type "PrimitiveComponent Object Reference") (OtherActor :type "Actor Object Reference") (OtherComp :type "PrimitiveComponent Object Reference") (OtherBodyIndex :type Integer) (bFromSweep :type Boolean) (SweepResult :type "HitResult Structure (by ref)"))
  (bind _bobbie_ref (`self.Bobbie_Ref`))
  (bind _bobbie_ref_2 (`self.Bobbie_Ref`))
  (bind _wbp_tableaudebord (`/Game/Widget/Hud/WBP_UI_Jeu.WBP_TableauDeBord` (`/Game/Blueprints/Boats/Bobbie/BP_BoatTemplate.UI_EnJeu` (`self.Bobbie_Ref`))))
  (if (== OtherActor (`GameplayStatics.GetPlayerPawn` 0))
    (bind _output_get (set `self.RalentissementBobbie?` true))
    (if (`self.NaufrageTutoriel?`)
      ;[1 1 1] Séquence pour un tutoriel sur les naufragés
      (if (`self.TutorielComplete`)
        (`|ExecutionSequence` :!label _label
          (:`then_0`
            (bind _output_get_2 (set `/Game/Blueprints/Boats/Bobbie/BP_BoatTemplate.DansLaZoneNaufrage` _output_get _bobbie_ref))
            (set `/Game/Blueprints/Boats/Bobbie/BP_BoatTemplate.RegardForce` _output_get_2 _bobbie_ref)
            (set `/Game/Blueprints/Boats/Bobbie/BP_BoatTemplate.CurrentNaufrage` self _bobbie_ref))
          (:`then_1`
            (if (`/Game/Blueprints/Boats/Bobbie/BP_BoatTemplate.Mobile?` _bobbie_ref)
              ;[1 1 1] Gestion de UI pour mobile lorsque Bobbie entre dans la zone pour sauver le naufragé
              (`/Game/Widget/Hud/WBP_TableauDeBord.AfficherTout` _wbp_tableaudebord)
              (`/Game/Widget/Hud/WBP_TableauDeBord.AfficherSauvetage` _wbp_tableaudebord)
              (else
                ;[1 1 1] Gestion de l'appartition du UI pour PC / Manette
                (`/Game/Widget/Hud/WBP_UI_Jeu.DansLaZoneSauvetage` (`/Game/Blueprints/Boats/Bobbie/BP_BoatTemplate.UI_EnJeu` _bobbie_ref))))))
        (else
          (`/Game/Widget/Hud/WBP_UI_Jeu.AjouterEcranTutoriel` (`/Game/Blueprints/Boats/Bobbie/BP_BoatTemplate.UI_EnJeu` _bobbie_ref_2) "NewEnumerator7")
          (`/Game/Blueprints/Boats/Bobbie/BP_BoatTemplate.DesactiverMouvements` _bobbie_ref_2)
          (set `self.TutorielComplete` true)))
      (else
        (goto _label)))))

(event `ContinuerTutoNaufrage`
  (goto _label))

(event `self.ZoneDeRalentissement.OnComponentEndOverlap`
  (params (OverlappedComponent :type "PrimitiveComponent Object Reference") (OtherActor :type "Actor Object Reference") (OtherComp :type "PrimitiveComponent Object Reference") (OtherBodyIndex :type Integer))
  (bind _bobbie_ref (`self.Bobbie_Ref`))
  (if (== OtherActor (`GameplayStatics.GetPlayerPawn` 0))
    (`|ExecutionSequence`
      (:`then_0`
        (bind _output_get (set `self.RalentissementBobbie?` false))
        (bind _output_get_2 (set `/Game/Blueprints/Boats/Bobbie/BP_BoatTemplate.DansLaZoneNaufrage` _output_get _bobbie_ref))
        (set `/Game/Blueprints/Boats/Bobbie/BP_BoatTemplate.RegardForce` _output_get_2 _bobbie_ref)
        (set `/Game/Blueprints/Boats/Bobbie/BP_BoatTemplate.CurrentNaufrage` null _bobbie_ref)
        (`/Game/Blueprints/Boats/Bobbie/BP_BoatTemplate.EteindreLumiere` _bobbie_ref))
      (:`then_1`
        (if (`/Game/Blueprints/Boats/Bobbie/BP_BoatTemplate.Mobile?` _bobbie_ref)
          ;[1 1 1] Lorsque Bobbie sort de la Zone de sauvetage le UI pour Mobile se cache.
          (`/Game/Widget/Hud/WBP_TableauDeBord.CacherTout` (`/Game/Widget/Hud/WBP_UI_Jeu.WBP_TableauDeBord` (`/Game/Blueprints/Boats/Bobbie/BP_BoatTemplate.UI_EnJeu` (`self.Bobbie_Ref`))))
          (else
            ;[1 1 1] Affichage du UI pour la version PC
            (`/Game/Widget/Hud/WBP_ModeVisee.CloseNotification` (`/Game/Widget/Hud/WBP_UI_Jeu.WBP_ModeVisee` (`/Game/Blueprints/Boats/Bobbie/BP_BoatTemplate.UI_EnJeu` _bobbie_ref)))))))))

(event `LancerFusee`
  ;[1 1 1] Apparition de la fusée de détresse
  (bind _returnvalue (`|SpawnActorFromClass` "/Game/Blueprints/Naufrages/BP_FuseeDetresse.BP_FuseeDetresse_C" (`KismetMathLibrary.MakeTransform` (+ (`self.K2_GetActorLocation`) (0.0 0.0 100.0))) "AlwaysSpawn" "MultiplyWithRoot" null null))
  (bind _output_get (set `self.FeuDetresse_Ref` _returnvalue))
  (set `/Game/Blueprints/Naufrages/BP_FuseeDetresse.HauteurFeuDetresse` (`self.Hauteur Feu Detresse`) _output_get)
  (`/Game/Blueprints/Naufrages/BP_FuseeDetresse.GetNaufrageParent` _output_get self)
  (`GameplayStatics.PlaySound2D` "/Game/Sfx/Sons/Effects/Sfx_Flare.Sfx_Flare" 1.0 1.0 0.0 null null)
  (`GameplayStatics.PlaySoundAtLocation` null (`self.K2_GetActorLocation` _output_get) (struct) 1.0 1.0 0.0 null null null null))

(event `CacherFumee`
  ;[1 1 1] Affiche le feu de détresse au sol ou le cache
  (`SceneComponent.SetVisibility` (`self.NS_GroundFlare`) false false)
  (`SceneComponent.SetVisibility` (`self.NS_GroundFlare1`) false false)
  (bind _asbp_fusee_detresse (cast `/Game/Blueprints/Naufrages/BP_FuseeDetresse` (`self.FeuDetresse_Ref`)))
  (`/Game/Blueprints/Naufrages/BP_FuseeDetresse.Cacher_AfficherFX` _asbp_fusee_detresse false))

(event `AfficherFumee`
  (bind _ns_groundflare (`self.NS_GroundFlare`))
  ;[1 1 1] Affiche le feu de détresse au sol ou le cache
  (`SceneComponent.SetVisibility` _ns_groundflare true false)
  (`SceneComponent.SetVisibility` (`self.NS_GroundFlare1`) true false)
  (`ActorComponent.Activate` _ns_groundflare true)
  (`ActorComponent.Activate` (`self.NS_GroundFlare1`) true)
  (bind _asbp_fusee_detresse (cast `/Game/Blueprints/Naufrages/BP_FuseeDetresse` (`self.FeuDetresse_Ref`)))
  (`/Game/Blueprints/Naufrages/BP_FuseeDetresse.Cacher_AfficherFX` _asbp_fusee_detresse true))

(event `ChangerObjectif`
  (`/Game/Blueprints/GuidingArrow/BP_FlecheGuide.PointSuivant` (`self.FlecheGuideObjectif_Ref`)))

(fn `CalculForceProportionelle`
  (params (ActorEnARalentir :type "/Game/Blueprints/Boats/Bobbie/BP_BoatTemplate Object Reference") (Distance :type "Float (double-precision)"))
  (returns (RetourDeForce :type "Float (double-precision)"))
  (bind (_datatablebateau_infos_nomdupersonnage _datatablebateau_infos_mesh _datatablebateau_infos_accessoire _datatablebateau_infos_positionaccessoire _datatablebateau_infos_sante _datatablebateau_infos_vitessebateau) (break `/Game/Blueprints/Boats/Bobbie/Struct_Boats` (`/Game/Blueprints/Boats/Bobbie/BP_BoatTemplate.DataTableBateau_Infos` ActorEnARalentir)))
  (return (* (`KismetMathLibrary.MapRangeClamped` (* (`PrimitiveComponent.GetMass` (`/Game/Blueprints/Boats/Bobbie/BP_BoatTemplate.SM_Bobbie` ActorEnARalentir)) (/ (`/Game/Blueprints/Boats/Bobbie/BP_BoatTemplate.VelociteGlobale` ActorEnARalentir) 1.0)) 0.0 (/ _datatablebateau_infos_vitessebateau 2.0) 0.0 1.0) Distance)))

(fn `NaufrageSecouru`
  (bind _bobbie_ref (`self.Bobbie_Ref`))
  (set `/Game/Blueprints/Boats/Bobbie/BP_BoatTemplate.IndexPersonneSecouru` (+ (`/Game/Blueprints/Boats/Bobbie/BP_BoatTemplate.IndexPersonneSecouru` _bobbie_ref) 1) _bobbie_ref)
  (`/Game/Widget/Hud/WBP_UI_Jeu.AjouterNaufrage` (`/Game/Blueprints/Boats/Bobbie/BP_BoatTemplate.UI_EnJeu` _bobbie_ref) ""))

(fn `PrintInfos`
  (params (NomDeValeur :type String) (Valeur :type String) (CouleurTexte :type "LinearColor Structure") (Duration :type "Float (single-precision)") (`Print À l'écran?` :type Boolean :default true))
  (`KismetSystemLibrary.PrintString` (`KismetStringLibrary.Concat_StrStr` NomDeValeur Valeur) false true CouleurTexte Duration))

(fn `UpdateZoneSauvetage`
  (params (Taille :type "Float (double-precision)"))
  (`SceneComponent.SetRelativeScale3D` (`self.Ring02`) (`KismetMathLibrary.MakeVector` Taille Taille 5.0)))

(fn `UserConstructionScript`
  (bind _taillezone (`self.TailleZone`))
  (`SceneComponent.SetRelativeScale3D` (`self.Ring02`) (`KismetMathLibrary.MakeVector` _taillezone _taillezone 4.0)))