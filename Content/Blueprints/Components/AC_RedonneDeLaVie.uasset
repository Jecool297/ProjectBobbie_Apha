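; AC_RedonneDeLaVie is a component that restores Bobbie's health, intended for his arrival at the Base for mission launch.
; Its ReparationBateau event skips players at or above maximum health, otherwise targeting either full health or current health plus a given amount.
; Each call applies a single delta-time FInterpTo step toward that target, so gradual healing needs repeated calls, then refreshes the in-game life UI.
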(event `ReparationBateau`
  (params (JoueurAGuerrir :type "/Game/Blueprints/Boats/Bobbie/BP_BoatTemplate Object Reference") (VieFull :type Boolean) (QuantiteDeVieRecu :type "Float (double-precision)"))
  (bind _santemax (`/Game/Blueprints/Boats/Bobbie/BP_BoatTemplate.SanteMax` JoueurAGuerrir))
  (bind _santebobbie (`/Game/Blueprints/Boats/Bobbie/BP_BoatTemplate.SanteBobbie` JoueurAGuerrir))
  ;[1 1 1] Redonne le max de sante à Bobbie lorsqu'il arrive à la Base pour le lancement de la mission
  (if (not (>= _santebobbie _santemax))
    (set `/Game/Blueprints/Boats/Bobbie/BP_BoatTemplate.SanteBobbie` (`KismetMathLibrary.FInterpTo` _santebobbie (`KismetMathLibrary.SelectFloat` _santemax (+ _santebobbie QuantiteDeVieRecu) VieFull) (`GameplayStatics.GetWorldDeltaSeconds`) 5.0) JoueurAGuerrir)
    (`/Game/Widget/Hud/WBP_UI_Jeu.MiseAJourVie` (`/Game/Blueprints/Boats/Bobbie/BP_BoatTemplate.UI_EnJeu` JoueurAGuerrir))))