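; Actor component that launches in-game events for the player's boat, currently a one-time Level Sequence cinematic.
; BeginPlay caches the player pawn as BP_BoatTemplate.
; LancerCinematique plays the sequence behind a DoOnce, disables boat movement, hides the in-game UI and binds FinCinematique to its end.
; FinCinematique calls GetAllNaufrage on the shipwreck list widget, shows the shipwreck help and re-enables movement; LancerAutre is an empty stub.
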(event `self.ReceiveBeginPlay`
  (bind _asbp_boat_template (cast `/Game/Blueprints/Boats/Bobbie/BP_BoatTemplate` (`GameplayStatics.GetPlayerPawn` 0)))
  (set `self.As BP Boat Template` _asbp_boat_template))

(event `LancerCinematique`
  (bind _as_bp_boat_template (`self.As BP Boat Template`))
  ;[1 1 1] Gère l'évènement du lancement de cinématique
  (`/Engine/EditorBlueprintResources/StandardMacros.DoOnce` false
    (:`Completed`
      (bind (_outactor _returnvalue) (`LevelSequencePlayer.CreateLevelSequencePlayer` (`self.LevelSequenceToPlay`)))
      (bind _output_get (set `self.SequenceEnCours` _returnvalue))
      (`MovieSceneSequencePlayer.Play` _output_get)
      (`/Game/Blueprints/Boats/Bobbie/BP_BoatTemplate.DesactiverMouvements` _as_bp_boat_template)
      (`/Game/Widget/Hud/WBP_UI_Jeu.CacherTout` (`/Game/Blueprints/Boats/Bobbie/BP_BoatTemplate.UI_EnJeu` _as_bp_boat_template))
      (add `MovieSceneSequencePlayer.OnFinished` _output_get (delegate `FinCinematique`)))))

(event `FinCinematique`
  (bind _as_bp_boat_template (`self.As BP Boat Template`))
  ;[1 1 1] Gère l'évènement du lancement de cinématique
  (`/Game/Widget/Hud/WBP_NaufrageList.GetAllNaufrage` (`/Game/Widget/Hud/WBP_UI_Jeu.WBP_NaufrageList` (`/Game/Blueprints/Boats/Bobbie/BP_BoatTemplate.UI_EnJeu` _as_bp_boat_template)))
  (`/Game/Widget/Hud/WBP_UI_Jeu.AffichageAideNaufrage` (`/Game/Blueprints/Boats/Bobbie/BP_BoatTemplate.UI_EnJeu` _as_bp_boat_template) "Visible")
  (`/Game/Blueprints/Boats/Bobbie/BP_BoatTemplate.ReactiverMouvements` _as_bp_boat_template))

(event `LancerAutre`)