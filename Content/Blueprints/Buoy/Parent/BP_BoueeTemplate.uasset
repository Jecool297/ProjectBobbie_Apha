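; Parent Blueprint for navigation buoys that return to their starting transform through ACRetourPosition when hit and can police a safe channel.
; The construction script passes Charpentes to a type switch setting mesh, capsule and mass, adding outer and inner trigger boxes for framework lateral buoys.
; With LimitationBouee enabled, the boat entering the outer box starts a looping timer that runs the boat's safety countdown until it reaches only the inner box.
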(event `self.ReceiveTick`
  (params (DeltaSeconds :type "Float (single-precision)"))
  (if (`self.ZoneSecuritaireAtteinte`)
    (bind _sortietimer (`self.Chronometre` false))
    (if (>= _sortietimer 5.0)
      _)
    (else
      (`self.Chronometre` true))))

(event `self.ReceiveBeginPlay`
  ;[1 1 1] Enregistrement de la position initiale
  (set `self.TransformationInitiale` (`self.GetTransform`))
  (bind _returnvalue (`GameplayStatics.GetActorOfClass` "/Game/Blueprints/Boats/Bobbie/BP_BoatTemplate.BP_BoatTemplate_C"))
  (set `self.As BP Boat Template` _returnvalue)
  (if (`self.LimitationBouee`)
    (bind _zoneexterieur (`self.ZoneExterieur`)
      (:`then`
        (add `PrimitiveComponent.OnComponentBeginOverlap` _zoneexterieur (delegate `SortieDeLaZoneSecuritataire`)))
      (:`else`))))

(event `self.Bouees.OnComponentHit`
  (params (HitComponent :type "PrimitiveComponent Object Reference") (OtherActor :type "Actor Object Reference") (OtherComp :type "PrimitiveComponent Object Reference") (NormalImpulse :type "Vector Structure") (Hit :type "HitResult Structure (by ref)"))
  ;[1 1 1] Retour à la position initial 3 secondes après l'impacte avec tout objet.
  (`/Game/Blueprints/Buoy/Parent/AC_RetourPosition.Collision_Hit` (`self.AC_RetourPosition`) (`self.TransformationInitiale`) (`self.Bouees`) (`self.DureeDeplacement`)))

(event `SortieDeLaZoneSecuritataire`
  (params (OverlappedComponent :type "PrimitiveComponent Object Reference") (OtherActor :type "Actor Object Reference") (OtherComp :type "PrimitiveComponent Object Reference") (OtherBodyIndex :type Integer) (bFromSweep :type Boolean) (SweepResult :type "HitResult Structure (by ref)"))
  (bind _as_bp_boat_template (`self.As BP Boat Template`))
  (if (and (== OtherActor _as_bp_boat_template) (not (`self.CompteurActif`)))
    (if (not (`/Game/Blueprints/Boats/Bobbie/BP_BoatTemplate.ChronoSecuriteLance` _as_bp_boat_template))
      (`self.LancementChrono`))))

(event `LancementChrono`
  ;[1 1 1] Ramèene le joueur sur le droit chemin après la fin du décompte d'un timer
  (set `self.CompteurActif` true)
  (`KismetSystemLibrary.K2_SetTimerDelegate` (delegate `CompteurActive`) 1.0 (`self.CompteurActif`)))

(event `CompteurActive`
  (bind _as_bp_boat_template (`self.As BP Boat Template`))
  ;[1 1 1] Ramèene le joueur sur le droit chemin après la fin du décompte d'un timer
  (if (`self.CompteurActif`)
    (if (`PrimitiveComponent.IsOverlappingActor` (`self.ZoneExterieur`) (`self.As BP Boat Template`))
      (`/Game/Blueprints/Boats/Bobbie/BP_BoatTemplate.LancementChronometreSecurite` _as_bp_boat_template self :!label _label)
      (elif (`PrimitiveComponent.IsOverlappingActor` (`self.ZoneInterieur`) (`self.As BP Boat Template`))
        (set `self.CompteurActif` false)
        (`/Game/Blueprints/Boats/Bobbie/BP_BoatTemplate.ArretChronometreSecurite` _as_bp_boat_template)
        (else
          (goto _label))))))

(fn `ChangerTypeDeBouees`
  (params (`Type de bouees` :type "/Game/Blueprints/Buoy/Enumerations/Enum_TypesBouees Enum (by ref)"))
  (locals (MassMaximum :type "Float (double-precision)" :default 2.0))
  (bind _bouees (`self.Bouees`))
  (bind _taillezoneexternebouee (`self.TailleZoneExterneBouee`))
  (bind _bouees_2 (`self.Bouees`))
  (bind _capsule (`self.Capsule`))
  (bind _capsule_2 (`self.Capsule`))
  (bind _capsule_3 (`self.Capsule`))
  (bind _capsule_4 (`self.Capsule`))
  (bind _bouees_3 (`self.Bouees`))
  (bind _bouees_4 (`self.Bouees`))
  (bind _taillezoneexternebouee_2 (`self.TailleZoneExterneBouee`))
  (bind _bouees_5 (`self.Bouees`))
  (bind _x (.x _taillezoneexternebouee_2))
  (bind _x_2 (.x _taillezoneexternebouee))
  (switch `/Game/Blueprints/Buoy/Enumerations/Enum_TypesBouees` `Type de bouees`
    (:`NewEnumerator0`
      (switch `/Game/Blueprints/Buoy/Enumerations/Enum_TypesBouees_Charpente` (`self.Type de bouees Charpente`)
        (:`NewEnumerator0`
          ;[1 1 1] Changement emtre les bouées à charpente (Plus lourde)
          (`StaticMeshComponent.SetStaticMesh` _bouees_3 "/Game/Art/Buoy/Danger/Framework/Mesh/SM_Bouees_SM_DangerIsole_Charpente.SM_Bouees_SM_DangerIsole_Charpente")
          (`CapsuleComponent.SetCapsuleSize` _capsule_3 70.0 200.0 true :!label _label))
        (:`NewEnumerator1`
          (`StaticMeshComponent.SetStaticMesh` _bouees_3 "/Game/Art/Buoy/Lateral/Green/Mesh/SM_LateralGreenFramework.SM_LateralGreenFramework")
          (bind _retourtiggerbox (`self.GreenTriggerZone` _taillezoneexternebouee_2 (+ (`KismetMathLibrary.MakeVector` _x 0.0 650.0) (`self.DistanceEntreLesZones`))))
          (set `self.ZoneExterieur` _retourtiggerbox)
          (bind _retourtiggerbox_2 (`self.YellowTriggerZone` _taillezoneexternebouee_2 (+ (`KismetMathLibrary.MakeVector` (* _x -1.0) 0.0 650.0) (* (-1.0 0.0 0.0) (`self.DistanceEntreLesZones`)))))
          (set `self.ZoneInterieur` _retourtiggerbox_2)
          (goto _label))
        (:`NewEnumerator2`
          (`StaticMeshComponent.SetStaticMesh` _bouees_3 "/Game/Art/Buoy/Lateral/Red/Mesh/SM_LateralRed_Framework.SM_LateralRed_Framework")
          (bind _retourtiggerbox_3 (`self.RedTriggerZone` _taillezoneexternebouee (+ (`KismetMathLibrary.MakeVector` _x_2 0.0 650.0) (`self.DistanceEntreLesZones`))))
          (set `self.ZoneExterieur` _retourtiggerbox_3)
          (bind _retourtiggerbox_4 (`self.YellowTriggerZone` _taillezoneexternebouee (+ (`KismetMathLibrary.MakeVector` (* _x_2 -1.0) 0.0 650.0) (* (`self.DistanceEntreLesZones`) (-1.0 0.0 0.0)))))
          (set `self.ZoneInterieur` _retourtiggerbox_4)
          (goto _label))
        (:`NewEnumerator3`
          (`StaticMeshComponent.SetStaticMesh` _bouees_3 "/Game/Art/Buoy/SafeWater/Mesh/SM_SafeWater_Framework.SM_SafeWater_Framework")
          (`CapsuleComponent.SetCapsuleSize` _capsule_3 55.0 160.0 true)))
      (`SceneComponent.K2_AddRelativeLocation` _capsule_3 (0.0 0.0 0.0) false false)
      (`PrimitiveComponent.SetMassScale` (`self.Bouees`) "None" (`local.MassMaximum`)))
    (:`NewEnumerator1`
      ;[1 1 1] Changement entre les bouées espar (Taille Moyenne )
      (switch `/Game/Blueprints/Buoy/Enumerations/Enum_TypesBouees_Espar` (`self.Type Bouees Espar`)
        (:`NewEnumerator0`
          (`StaticMeshComponent.SetStaticMesh` _bouees_2 "/Game/Art/Buoy/Danger/Espar/Mesh/SM_Bouees_SM_DangerIsole_Espar.SM_Bouees_SM_DangerIsole_Espar")
          (`CapsuleComponent.SetCapsuleSize` _capsule_2 35.0 75.0 true :!label _label_2)
          (`SceneComponent.K2_AddRelativeLocation` _capsule_2 (0.0 0.0 -150.0) false false))
        (:`NewEnumerator1`
          (`StaticMeshComponent.SetStaticMesh` _bouees_2 "/Game/Art/Buoy/Lateral/Green/Mesh/SM_LateralGreenEspar.SM_LateralGreenEspar")
          (goto _label_2))
        (:`NewEnumerator2`
          (`StaticMeshComponent.SetStaticMesh` _bouees_2 "/Game/Art/Buoy/Lateral/Red/Mesh/SM_LateralRed_Biffurcation.SM_LateralRed_Biffurcation")
          (goto _label_2))
        (:`NewEnumerator3`
          (`StaticMeshComponent.SetStaticMesh` _bouees_2 "/Game/Art/Buoy/SafeWater/Mesh/SM_SafeWater_Espar.SM_SafeWater_Espar"))
        (:`NewEnumerator8`
          (`StaticMeshComponent.SetStaticMesh` _bouees_2 "/Game/Art/Buoy/Other/SlowSign/SM_BoueesSlow_Espar.SM_BoueesSlow_Espar")))
      (`PrimitiveComponent.SetMassScale` (`self.Bouees`) "None" (/ (`local.MassMaximum`) 2.0)))
    (:`NewEnumerator2`
      ;[1 1 1] Changements entre les type de bouées cardinales
      (switch `/Game/Blueprints/Buoy/Enumerations/Enum_TypesBouees_Cardinales` (`self.Type de bouees Cardinales`)
        (:`NewEnumerator0`
          (`StaticMeshComponent.SetStaticMesh` _bouees_5 "/Game/Art/Buoy/Cardinals/Mesh/SM_Bouee_Cardinales_Nord.SM_Bouee_Cardinales_Nord"))
        (:`NewEnumerator1`
          (`StaticMeshComponent.SetStaticMesh` _bouees_5 "/Game/Art/Buoy/Cardinals/Mesh/SM_Bouee_Cardinales_Sud.SM_Bouee_Cardinales_Sud"))
        (:`NewEnumerator2`
          (`StaticMeshComponent.SetStaticMesh` _bouees_5 "/Game/Art/Buoy/Cardinals/Mesh/SM_Bouees_Cardinales_Ouest.SM_Bouees_Cardinales_Ouest"))
        (:`NewEnumerator3`
          (`StaticMeshComponent.SetStaticMesh` _bouees_5 "/Game/Art/Buoy/Cardinals/Mesh/SM_Bouees_Cardinales_Est.SM_Bouees_Cardinales_Est")))
      (`CapsuleComponent.SetCapsuleSize` _capsule_4 55.0 160.0 true)
      (`SceneComponent.K2_AddRelativeLocation` _capsule_4 (0.0 0.0 0.0) false false)
      (`PrimitiveComponent.SetMassScale` (`self.Bouees`) "None" (`local.MassMaximum`)))
    (:`NewEnumerator8`
      ;[1 1 1] Changements entre les type de bouées cardinales
      (switch `/Game/Blueprints/Buoy/Enumerations/Enum_TypesBouees_Biffurcation` (`self.TypeBoueesBiffurcation`)
        (:`NewEnumerator0`
          (`StaticMeshComponent.SetStaticMesh` _bouees_4 "/Game/Art/Buoy/Lateral/Red/Mesh/SM_LateralRed_Biffurcation.SM_LateralRed_Biffurcation"))
        (:`NewEnumerator1`
          (`StaticMeshComponent.SetStaticMesh` _bouees_4 "/Game/Art/Buoy/Lateral/Green/Mesh/SM_LateralGreenBiffurcation.SM_LateralGreenBiffurcation"))
        (:`NewEnumerator2`
          (`StaticMeshComponent.SetStaticMesh` _bouees_4 "/Game/Art/Buoy/Lateral/Green/Mesh/SM_LateralGreenFramework.SM_LateralGreenFramework"))
        (:`NewEnumerator3`
          (`StaticMeshComponent.SetStaticMesh` _bouees "/Game/Art/Buoy/Lateral/Red/Mesh/SM_LateralRed_Biffurcation.SM_LateralRed_Biffurcation"))
        (:`NewEnumerator8`
          (`StaticMeshComponent.SetStaticMesh` _bouees "/Game/Art/Buoy/Lateral/Green/Mesh/SM_LateralGreenBiffurcation.SM_LateralGreenBiffurcation"))
        (:`NewEnumerator9`
          (`StaticMeshComponent.SetStaticMesh` _bouees "/Game/Art/Buoy/Lateral/Red/Mesh/SM_LateralRed_Framework.SM_LateralRed_Framework")))
      (`CapsuleComponent.SetCapsuleSize` _capsule 35.0 55.0 true)
      (`SceneComponent.K2_AddRelativeLocation` _capsule (0.0 0.0 -250.0) false false)
      (`PrimitiveComponent.SetMassScale` (`self.Bouees`) "None" (`local.MassMaximum`)))))

(fn `Chronometre`
  (params (ResetChrono :type Boolean))
  (returns (SortieTimer :type "Float (double-precision)"))
  (if ResetChrono
    (set `self.Timer Interne` 0.0)
    (else
      (bind _output_get (set `self.Timer Interne` (+ (`GameplayStatics.GetWorldDeltaSeconds`) (`self.Timer Interne`))))
      (return _output_get))))

(fn `GreenTriggerZone`
  (params (TailleTriggerBox :type "Vector Structure") (PositionTriggerBox :type "Vector Structure"))
  (returns (RetourTiggerBox :type "BoxComponent Object Reference"))
  (bind _returnvalue (`AddComponent|NODE_AddBoxComponent-4` :`RelativeTransform` (`KismetMathLibrary.MakeTransform` (+ PositionTriggerBox (`self.PositionZones`)))))
  (`SceneComponent.K2_AttachToComponent` _returnvalue (`self.Bouees`) "None" "KeepRelative" "KeepRelative" "KeepRelative" true)
  (`BoxComponent.SetBoxExtent` _returnvalue TailleTriggerBox true)
  (return _returnvalue))

(fn `PrintInfos`
  (params (NomDeValeur :type String) (Valeur :type String) (CouleurTexte :type "LinearColor Structure") (Duration :type "Float (single-precision)") (`Print À l'écran?` :type Boolean :default true))
  (`KismetSystemLibrary.PrintString` (`KismetStringLibrary.Concat_StrStr` NomDeValeur Valeur) false true CouleurTexte Duration))

(fn `RedTriggerZone`
  (params (TailleTriggerBox :type "Vector Structure") (PositionTriggerBox :type "Vector Structure"))
  (returns (RetourTiggerBox :type "BoxComponent Object Reference"))
  (bind _returnvalue (`AddComponent|NODE_AddBoxComponent-0` :`RelativeTransform` (`KismetMathLibrary.MakeTransform` (+ PositionTriggerBox (`self.PositionZones`)))))
  (`SceneComponent.K2_AttachToComponent` _returnvalue (`self.Bouees`) "None" "KeepRelative" "KeepRelative" "KeepRelative" true)
  (`BoxComponent.SetBoxExtent` _returnvalue TailleTriggerBox true)
  (return _returnvalue))

(fn `UserConstructionScript`
  (`self.ChangerTypeDeBouees` "NewEnumerator0"))

(fn `YellowTriggerZone`
  (params (TailleTriggerBox :type "Vector Structure") (PositionTriggerBox :type "Vector Structure"))
  (returns (RetourTiggerBox :type "BoxComponent Object Reference"))
  (bind _returnvalue (`AddComponent|NODE_AddBoxComponent-5` :`RelativeTransform` (`KismetMathLibrary.MakeTransform` (+ PositionTriggerBox (`self.PositionZones`)))))
  (`SceneComponent.K2_AttachToComponent` _returnvalue (`self.Bouees`) "None" "KeepRelative" "KeepRelative" "KeepRelative" true)
  (`BoxComponent.SetBoxExtent` _returnvalue TailleTriggerBox true)
  (return _returnvalue))