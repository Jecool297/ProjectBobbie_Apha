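; Blueprint function library of shared UI helpers for menus, help popups and player boat data.
; AjoutElementMenu collects a parent widget's level buttons into an array, then UpdateSelection tints the indexed one as highlighted and the rest as deselected.
; BoiteDialogue spawns a configurable BP_PopupAide on the viewport.
; Other helpers add frame delta to a resettable timer and return the player's BP_BoatTemplate with its data-table info.
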(fn `AjoutElementMenu`
  (params (ItemsDuMenu :type "Array of Widget Object Reference (by ref)") (`Widget Parent` :type "PanelWidget Object Reference") (Index :type Integer) (HoverColor :type "LinearColor Structure") (DeselectColor :type "LinearColor Structure"))
  (for _array_element (`PanelWidget.GetAllChildren` `Widget Parent`)
    (bind _aswbp_button_niveau (cast `/Game/Widget/Buttons/WBP_ButtonNiveau` _array_element))
    (`KismetArrayLibrary.Array_Add` ItemsDuMenu _aswbp_button_niveau))
  (`self.UpdateSelection` HoverColor DeselectColor ItemsDuMenu Index))

(fn `BoiteDialogue`
  (params (`PourQuitter?` :type Boolean) (`Timer?` :type Boolean) (PourCinematique :type Boolean) (`SetCustomImage?` :type Boolean) (CustomImage :type "Object Object Reference") (DelaiTimer :type "Float (double-precision)") (TaillePolice :type "Float (single-precision)") (`Texte A Afficher` :type Text))
  (returns (WidgetAffiche :type "/Game/Widget/Hud/BP_PopupAide Object Reference"))
  (bind _returnvalue (`|CreateWidget` "/Game/Widget/Hud/BP_PopupAide.BP_PopupAide_C" null `PourQuitter?` DelaiTimer PourCinematique `Texte A Afficher` TaillePolice CustomImage `SetCustomImage?` `Timer?`))
  (`UserWidget.AddToViewport` _returnvalue 10)
  (return _returnvalue))

(fn `CallDataTable`
  (returns (Ref_Joueur :type "/Game/Blueprints/Boats/Bobbie/BP_BoatTemplate Object Reference") (`Info Perso Choisi` :type "/Game/Blueprints/Boats/Bobbie/Struct_Boats Structure"))
  (locals (`As BP Boat Template` :type "/Game/Blueprints/Boats/Bobbie/BP_BoatTemplate Object Reference"))
  (bind _asbp_boat_template (cast `/Game/Blueprints/Boats/Bobbie/BP_BoatTemplate` (`GameplayStatics.GetPlayerPawn` null)))
  (bind _output_get (set `local.As BP Boat Template` _asbp_boat_template))
  (return _output_get (`/Game/Blueprints/Boats/Bobbie/BP_BoatTemplate.DataTableBateau_Infos` _output_get)))

(fn `ChronometreTempsEcoule`
  (params (`ResetTimer?` :type Boolean))
  (returns (SortieTimer :type "Float (double-precision)"))
  (locals (TimerInterne :type "Float (double-precision)") (NewLocalVar :type Boolean))
  (if `ResetTimer?`
    (set `local.TimerInterne` 0.0)
    (else
      (bind _output_get (set `local.TimerInterne` (+ (`GameplayStatics.GetWorldDeltaSeconds` null) (`local.TimerInterne`))))
      (return _output_get))))

(fn `UpdateSelection`
  (params (HoverColor :type "LinearColor Structure") (DeselectColor :type "LinearColor Structure") (ItemsDuMenu :type "Array of Widget Object Reference") (Index :type Integer))
  (for (_array_element _array_index) ItemsDuMenu
    (bind _asbutton (cast `Button` _array_element))
    (if (== _array_index Index)
      (`Button.SetColorAndOpacity` _asbutton HoverColor)
      (else
        (`Button.SetColorAndOpacity` _asbutton DeselectColor)))))