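; Boat base that combines an optional repair dock, a castaway rescue mission and its drop-off zone.
; Overlapping the repair trigger while damaged locks movement, while timelines drive healing and dynamic-material feedback.
; A box overlap or first tutorial repair launches the mission, revealing castaways filtered from an actor list.
; Returning with all of them plays a completion sequence, advances the guide arrow and optionally shows the victory message.
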(event `self.ReceiveBeginPlay`
  (bind _naufragea_recuperer (`self.NaufrageA Recuperer`))
  ;[1 1 1] Référence à Bobbie
  (bind _asbp_boat_template (cast `/Game/Blueprints/Boats/Bobbie/BP_BoatTemplate` (`GameplayStatics.GetPlayerPawn` 0)))
  (set `self.Bobbie_Ref` _asbp_boat_template)
  (bind _returnvalue (`GameplayStatics.GetActorOfClass` "/Game/Blueprints/GuidingArrow/BP_FlecheGuide.BP_FlecheGuide_C"))
  (set `self.Ref_FlecheGuide` _returnvalue)
  (bind _aswbp_compte_naufrage (cast `/Game/Widget/Mission/WBP_CompteNaufrage` (`WidgetComponent.GetWidget` (`self.Widget`))))
  (set `self.As WBP Compte Naufrage` _aswbp_compte_naufrage)
  (`|ExecutionSequence`
    (:`then_0`
      (bind _returnvalue_2 (`PrimitiveComponent.CreateDynamicMaterialInstance` (`self.Croix`) 0 "/Game/Material/Master/Vfx/M_Zone.M_Zone" "None"))
      (bind _output_get (set `self.MaterielZoneSoin` _returnvalue_2))
      (`PrimitiveComponent.SetMaterial` (`self.ZoneReparation`) 0 _output_get)
      (`PrimitiveComponent.SetMaterial` (`self.Croix`) 0 _output_get))
    (:`then_1`
      (bind _returnvalue_3 (`PrimitiveComponent.CreateDynamicMaterialInstance` (`self.ZoneDepotNaufrage`) 0 "/Game/Material/Master/Vfx/M_Zone.M_Zone" "None"))
      (bind _output_get_2 (set `self.MaterielZoneNaufrage ` _returnvalue_3))
      (`PrimitiveComponent.SetMaterial` (`self.ZoneNaufrage`) 0 _output_get_2))
    (:`then_2`
      ;[1 1 1] Vérifie que les Actor entrée dans la liste de la base est bien un naufragé. Dans le cas ou ce n'en est pas un, il sera supprimé de cette liste ne laissant que les naufragés
      (for _array_element _naufragea_recuperer
        ;;[1 1 1] Vérification que les acteurs sont bien de la classe naufragé(Effectué en loop selon la longueur de la liste entrée)
        (if (!= (`GameplayStatics.GetObjectClass` _array_element) "/Game/Blueprints/Naufrages/BP_NaufrageV2.BP_NaufrageV2_C")
          ;;[1 1 1] Retrait des acteurs non-naufragés du array(S'il y a lieu)
          (`KismetArrayLibrary.Array_RemoveItem` (`self.NaufrageA Recuperer`) _array_element)))
      ;[1 1 1] Une fois la vérification effectué, le nombre de naufragé requis s'applique automatiquement
      (set `self.PersonnesRequises` (`KismetArrayLibrary.Array_Length` _naufragea_recuperer)))
    (:`then_3`
      (`self.SetCouleurZone` (`self.ZoneReparation`)))))

(event `InitiationDesNaufrages`
  ;[1 1 1] Fait apparaitre les naufragés à leurs endroit respectif (Position des ''Arrows'' du BP_Base)
  ;;[1 1 1] Mets à jour la taille de la zone dans laquelle le bateau dois se positionner pour initier le sauvetage. Le rayon de Zone Naufrage défini dans l'éditeur dans le même ordre que le setup des naufragés
  (for (_array_element _array_index) (`self.NaufrageA Recuperer`)
    (bind _asbp_naufrage_v2 (cast `/Game/Blueprints/Naufrages/BP_NaufrageV2` _array_element)
      (:`then`
        (`/Engine/EditorBlueprintResources/StandardMacros.IsValid` _asbp_naufrage_v2
          (:`Is Valid`
            (`SceneComponent.SetHiddenInGame` (`Actor.RootComponent` _asbp_naufrage_v2) false true)
            (set `self.MissionLance?` true)
            (`/Game/Blueprints/Naufrages/BP_NaufrageV2.UpdateZoneSauvetage` _asbp_naufrage_v2 (`|GetArrayItem` (`self.RayonDeZoneNaufrage`) _array_index)))))
      (:`CastFailed`
        (`KismetSystemLibrary.PrintString` "ERROR")))))

(event `self.TriggerZoneReparation.OnComponentBeginOverlap`
  (params (OverlappedComponent :type "PrimitiveComponent Object Reference") (OtherActor :type "Actor Object Reference") (OtherComp :type "PrimitiveComponent Object Reference") (OtherBodyIndex :type Integer) (bFromSweep :type Boolean) (SweepResult :type "HitResult Structure (by ref)"))
  (bind _bobbie_ref (`self.Bobbie_Ref`))
  (bind _bobbie_ref_2 (`self.Bobbie_Ref`))
  ;[1 1 1] Transition des couleur lorsque le bateau se positionne pour une réparation
  (if (== OtherActor _bobbie_ref)
    (set `self.DansLaZoneReparation` true)
    (if (not (`KismetMathLibrary.NearlyEqual_FloatFloat` (`/Game/Blueprints/Boats/Bobbie/BP_BoatTemplate.SanteBobbie` _bobbie_ref) (`/Game/Blueprints/Boats/Bobbie/BP_BoatTemplate.SanteMax` _bobbie_ref)))
      (`KismetSystemLibrary.Delay` 0.2)
      (`/Game/Blueprints/Boats/Bobbie/BP_BoatTemplate.DesactiverMouvements` _bobbie_ref)
      (bind (_direction _newtrack_1) (`Timeline|DelaiReparation` :!label _label)
        (:`Update`
          (`MeshComponent.SetVectorParameterValueOnMaterials` (`self.Croix`) "Color" _newtrack_1)
          (`MeshComponent.SetVectorParameterValueOnMaterials` (`self.ZoneReparation`) "Color" _newtrack_1))
        (:`Finished`
          (if (`self.DansLaZoneReparation`)
            (set `self.Reparation` true)
            (bind (_direction_2 _progresreparation) (`Timeline|ReparationEnCours` :!via `PlayFromStart` :!label _label_2)
              (:`Update`
                (`MeshComponent.SetScalarParameterValueOnMaterials` (`self.Croix`) "ProgresReparation" _progresreparation)
                (`MeshComponent.SetScalarParameterValueOnMaterials` (`self.ZoneReparation`) "ProgresReparation" _progresreparation)
                (`/Game/Blueprints/Components/AC_RedonneDeLaVie.ReparationBateau` (`self.AC_RedonneDeLaVie`) _bobbie_ref_2 true 0.0))
              (:`Finished`
                (set `self.Reparation` false)
                (if (and (`self.TutorielSoin?`) (`self.PremierSoin`))
                  (`self.LancementMission`)
                  (set `self.PremierSoin` false)
                  (set `self.TutorielSoin?` false)
                  (else
                    (`/Game/Blueprints/Boats/Bobbie/BP_BoatTemplate.ReactiverMouvements` _bobbie_ref_2))))))))
      (else
        (`/Game/Widget/Hud/WBP_LevierVitesse.SnapLevierNeutre` (`/Game/Widget/Hud/WBP_UI_Jeu.WBP_LevierVitesse` (`/Game/Blueprints/Boats/Bobbie/BP_BoatTemplate.UI_EnJeu` _bobbie_ref)))))))

(event `LancementMission`
  (`/Game/Blueprints/Components/AC_LancementEvents.LancerCinematique` (`self.AC_LancementEvents`))
  (set `/Game/Blueprints/Boats/Bobbie/BP_BoatTemplate.CurrentBase` self (`self.Bobbie_Ref`))
  (`/Game/Widget/Mission/WBP_CompteNaufrage.SetNombrePersonneRequise` (`self.As WBP Compte Naufrage`) (`KismetTextLibrary.Conv_IntToText` (`self.PersonnesRequises`)))
  (`self.InitiationDesNaufrages`))

(event `self.TriggerZoneReparation.OnComponentEndOverlap`
  (params (OverlappedComponent :type "PrimitiveComponent Object Reference") (OtherActor :type "Actor Object Reference") (OtherComp :type "PrimitiveComponent Object Reference") (OtherBodyIndex :type Integer))
  ;[1 1 1] Transition des couleur lorsque le bateau se positionne pour une réparation
  (if (== OtherActor (`self.Bobbie_Ref`))
    (set `self.DansLaZoneReparation` false)
    (set `self.Reparation` false)
    (`/Game/Blueprints/Boats/Bobbie/BP_BoatTemplate.ReactiverMouvements` (`self.Bobbie_Ref`))
    (`|ExecutionSequence`
      (:`then_0`
        (goto _label :!via `Reverse`))
      (:`then_1`
        (`TimelineComponent.SetNewTime` (`self.ReparationEnCours`) 0.0)
        (goto _label_2 :!via `Stop`)))))

(event `self.Box.OnComponentBeginOverlap`
  (params (OverlappedComponent :type "PrimitiveComponent Object Reference") (OtherActor :type "Actor Object Reference") (OtherComp :type "PrimitiveComponent Object Reference") (OtherBodyIndex :type Integer) (bFromSweep :type Boolean) (SweepResult :type "HitResult Structure (by ref)"))
  (if (and (== OtherActor (`self.Bobbie_Ref`)) (not (`self.TutorielSoin?`)))
    (`/Engine/EditorBlueprintResources/StandardMacros.DoOnce` false
      (:`Completed`
        (`self.LancementMission`)))))

(event `self.ReceiveTick`
  (params (DeltaSeconds :type "Float (single-precision)"))
  (`|ExecutionSequence`
    (:`then_0`
      ;[1 1 1] Rotation de la croix toujours face au joueur
      (if (`self.QuaiDeReparation?`)
        (bind _bobbie_ref (`self.Bobbie_Ref`)
          (:`then`
            (`self.LookAtActor` _bobbie_ref (`self.Croix`) 90.0))
          (:`else`))))
    (:`then_1`
      (bind _bobbie_ref_2 (`self.Bobbie_Ref`)
        (:`then`
          (`self.LookAtActor` _bobbie_ref_2 (`self.Widget`) 0.0 0.0 90.0))
        (:`else`)))))

(event `self.ZoneDepotNaufrage.OnComponentBeginOverlap`
  (params (OverlappedComponent :type "PrimitiveComponent Object Reference") (OtherActor :type "Actor Object Reference") (OtherComp :type "PrimitiveComponent Object Reference") (OtherBodyIndex :type Integer) (bFromSweep :type Boolean) (SweepResult :type "HitResult Structure (by ref)"))
  (bind _bobbie_ref (`self.Bobbie_Ref`))
  (bind _bobbie_ref_2 (`self.Bobbie_Ref`))
  (bind _returnvalue (and (== OtherActor _bobbie_ref) (== (`/Game/Blueprints/Boats/Bobbie/BP_BoatTemplate.IndexPersonneSecouru` _bobbie_ref) (`self.PersonnesRequises`))))
  ;[1 1 1] Lancement de la séquence finale lorsque la mission est accompli
  (`/Engine/EditorBlueprintResources/StandardMacros.IsValid` _bobbie_ref
    (:`Is Valid`
      (if _returnvalue
        (`/Engine/EditorBlueprintResources/StandardMacros.DoOnce` false
          (:`Completed`
            (`|ExecutionSequence`
              (:`then_0`
                (bind (_outactor _returnvalue_2) (`LevelSequencePlayer.CreateLevelSequencePlayer` (`self.CinematiqueMissionAccompli`) :!label _label_3))
                (bind _output_get (set `self.SequenceMissionAccompliEncour` _returnvalue_2))
                (`MovieSceneSequencePlayer.Play` _output_get)
                (`/Game/Blueprints/Boats/Bobbie/BP_BoatTemplate.DesactiverMouvements` _bobbie_ref_2)
                (`/Game/Widget/Hud/WBP_NaufrageList.EffacerNaufrage` (`/Game/Widget/Hud/WBP_UI_Jeu.WBP_NaufrageList` (`/Game/Blueprints/Boats/Bobbie/BP_BoatTemplate.UI_EnJeu` _bobbie_ref_2)))
                (set `/Game/Blueprints/Boats/Bobbie/BP_BoatTemplate.IndexPersonneSecouru` 0 _bobbie_ref_2)
                (bind _ref_flecheguide (`self.Ref_FlecheGuide`)
                  (:`then`
                    (`/Game/Blueprints/GuidingArrow/BP_FlecheGuide.PointSuivant` _ref_flecheguide))
                  (:`else`
                    _))
                (`self.AffichageZoneNaufrage` false)
                (if (`self.MissionFinDeJeu`)
                  (`KismetSystemLibrary.Delay` 1.0)
                  (`/Game/Widget/Hud/WBP_UI_Jeu.MessageFinVictoire` (`/Game/Blueprints/Boats/Bobbie/BP_BoatTemplate.UI_EnJeu` (`self.Bobbie_Ref`)) "Visible" (`KismetMathLibrary.SelectText` "Mission Accomplie!\n\nFélicitation!\nVous avez réussi à sauver tout le monde!" "Mission Accomplie!\n\nFélicitation!\nVous avez réussi à sauver tout le monde!" _returnvalue))))
              (:`then_1`
                (bind _returnvalue_3 (`GameplayStatics.GetActorOfClass` "/Game/Blueprints/Boats/BateauAMoteur/BP_BlockingBoat.BP_BlockingBoat_C"))
                (bind _boat (`/Game/Blueprints/Boats/BateauAMoteur/BP_BlockingBoat.Boat` _returnvalue_3))
                (`/Engine/EditorBlueprintResources/StandardMacros.IsValid` _boat
                  (:`Is Valid`
                    (`PrimitiveComponent.SetConstraintMode` _boat "None")))))))))))

(event `MissionAccompli`
  ;[1 1 1] Lancement de la séquence finale lorsque la mission est accompli
  (goto _label_3))

(event `SetCouleurZone`
  (params (ZoneAffecte :type "MeshComponent Object Reference") (`Rouge?` :type Boolean))
  (`MeshComponent.SetVectorParameterValueOnMaterials` ZoneAffecte "Color" (`KismetMathLibrary.SelectVector` (1.0 0.0 0.0) (0.0 1.0 0.0) `Rouge?`)))

(event `AffichageZoneNaufrage`
  (params (bNewVisibility :type Boolean))
  (`SceneComponent.SetVisibility` (`self.ZoneNaufrage`) bNewVisibility true))

(fn `LookAtActor`
  (params (`FromActor ` :type "Actor Object Reference") (ActorToMove :type "SceneComponent Object Reference") (`X Modifier` :type "Float (single-precision)") (`Y Modifier` :type "Float (single-precision)") (`Z Modifier` :type "Float (double-precision)"))
  (bind (_returnvalue_roll _returnvalue_pitch _returnvalue_yaw) (`KismetMathLibrary.BreakRotator` (`KismetMathLibrary.FindLookAtRotation` (`SceneComponent.K2_GetComponentLocation` ActorToMove) (`self.K2_GetActorLocation` `FromActor `))))
  (`SceneComponent.K2_SetRelativeRotation` ActorToMove (`KismetMathLibrary.MakeRotator` `X Modifier` `Y Modifier` (+ _returnvalue_yaw `Z Modifier`)) false false))

(fn `UserConstructionScript`
  (bind _quaidereparation_ (`self.QuaiDeReparation?`))
  (bind _quai (`self.Quai`))
  (bind _triggerzonereparation (`self.TriggerZoneReparation`))
  (`|ExecutionSequence`
    (:`then_0`
      (`SceneComponent.SetHiddenInGame` _quai (not _quaidereparation_) true)
      (`SceneComponent.SetVisibility` _quai _quaidereparation_ true)
      (`SceneComponent.SetHiddenInGame` _triggerzonereparation true false)
      (`SceneComponent.SetVisibility` _triggerzonereparation false false)
      (`MeshComponent.SetScalarParameterValueOnMaterials` (`self.Croix`) "ProgresReparation" -0.5)
      (`MeshComponent.SetScalarParameterValueOnMaterials` (`self.ZoneReparation`) "ProgresReparation" -0.5))
    (:`then_1`
      (`self.SetCouleurZone` (`self.Croix`))
      (`self.SetCouleurZone` (`self.ZoneReparation`))
      (`SceneComponent.SetVisibility` (`self.Billboard`) false true)
      (`SceneComponent.SetVisibility` (`self.ZoneDepotNaufrage`) false true)
      (`SceneComponent.SetVisibility` (`self.ZoneNaufrage`) false true))))