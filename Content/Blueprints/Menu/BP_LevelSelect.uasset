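; BP_LevelSelect is a menu actor that marks the selected level by showing one of four level components.
; The construction script hides all four, and BeginPlay stores them in an ordered array.
; AfficherNiveauSelectionne shows the component at the given index and hides the others.
; AffichageFleche, named for arrow display, sets the visibility of all four at once.
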(event `self.ReceiveTick`
  (params (DeltaSeconds :type "Float (single-precision)")))

(event `self.ReceiveBeginPlay`
  (set `self.PositionNiveaux` (`|MakeArray` (`self.Level00`) (`self.Level01`) (`self.Level02`) (`self.Level03`))))

(event `AfficherNiveauSelectionne`
  (params (Index :type Integer))
  (bind _output_get (set `self.NiveauActuellementSelectionne` (`|GetArrayItem` (`self.PositionNiveaux`) Index)))
  (`SceneComponent.SetVisibility` _output_get true false)
  (for _array_element (`self.PositionNiveaux`)
    (if (!= _array_element (`self.NiveauActuellementSelectionne`))
      (`SceneComponent.SetVisibility` _array_element false false))))

(event `AffichageFleche`
  (params (bNewVisibility :type Boolean))
  (`SceneComponent.SetVisibility` (`self.Level01`) bNewVisibility false)
  (`SceneComponent.SetVisibility` (`self.Level02`) bNewVisibility false)
  (`SceneComponent.SetVisibility` (`self.Level03`) bNewVisibility false)
  (`SceneComponent.SetVisibility` (`self.Level00`) bNewVisibility false))

(fn `UserConstructionScript`
  (`SceneComponent.SetVisibility` (`self.Level01`) false false)
  (`SceneComponent.SetVisibility` (`self.Level00`) false false)
  (`SceneComponent.SetVisibility` (`self.Level02`) false false)
  (`SceneComponent.SetVisibility` (`self.Level03`) false false))