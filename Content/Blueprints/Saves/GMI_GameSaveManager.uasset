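; GMI_GameSaveManager is a save manager skeleton for character appearance, difficulty, collectables, and health and speed upgrades.
; Only SaveApparence stores data, copying the chosen boat type into InfoPersoChoisi.
; Initialisation, collectable and upgrade events are empty, and SetupDifficulte only unpacks its struct.
; The separate SetupDatatable helper checks that an "InfosPartie" row exists, then returns the table and the row name at the given index.
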(event `Initialisation`)

(event `SaveApparence`
  (params (TypeDeBatea :type "/Game/Blueprints/Boats/Bobbie/Struct_Boats Structure"))
  (set `self.InfoPersoChoisi` TypeDeBatea))

(event `SetupDifficulte`
  (params (`Struct Infos Partie Difficulte` :type "/Game/Blueprints/GameModes/Enum_Difficulte Enum" :default "NewEnumerator0"))
  (switch `/Game/Blueprints/GameModes/Enum_Difficulte` `Struct Infos Partie Difficulte`))

(event `SaveCollectable`)

(event `AmeliorationVie`
  (params (AmeliorationVie :type "Float (double-precision)")))

(event `AmeliorationVitesse`
  (params (AmeliorationVitesse :type "Float (double-precision)")))

(fn `SetupDatatable`
  (params (DataTableToSet :type "DataTable Object Reference") (RowIndex :type Integer))
  (returns (OutputPin :type "DataTable Object Reference") (Output :type Name))
  (bind _returnvalue (`DataTableFunctionLibrary.DoesDataTableRowExist` DataTableToSet "InfosPartie"))
  (if _returnvalue
    (bind _outrownames (`DataTableFunctionLibrary.GetDataTableRowNames` DataTableToSet))
    (return DataTableToSet (`|GetArrayItem` _outrownames RowIndex))))